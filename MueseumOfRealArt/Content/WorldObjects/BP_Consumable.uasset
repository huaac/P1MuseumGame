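; BP_Consumable is a world pickup that heals the player on touch.
; When the player character overlaps PickUpCollision and its health differs from max, it calls HealPlayer on the character's DamageComponent with a fixed amount, then destroys itself.
; At full health the pickup stays in place.
; The construction script gives the Sphere a glowing dynamic instance of the debug color material.
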(event OnComponentBeginOverlap(PickUpCollision)
  (params (OverlappedComponent :type Primitive%20Component%20Object%20Reference) (OtherActor :type Actor%20Object%20Reference) (OtherComp :type Primitive%20Component%20Object%20Reference) (OtherBodyIndex :type Integer) (bFromSweep :type Boolean) (SweepResult :type Hit%20Result%20Structure%20%28by%20ref%29))
  (bind _returnvalue (Game|GetPlayerCharacter 0))
  (bind _returnvalue_2 (Actor|GetComponentbyClass _returnvalue "/Game/Characters/DamageComponent.DamageComponent_C"))
  (bind _playercharacter (Variables|/Game/Characters/DamageComponent.DamageComponent_C|GetPlayerCharacter _returnvalue_2))
  (if (== OtherActor (Game|GetPlayerCharacter 0))
    (if (!= (Variables|/Game/ThirdPerson/Blueprints/BP_ThirdPersonCharacter.BP_ThirdPersonCharacter_C|GetCurrentHealth _playercharacter) (Variables|/Game/ThirdPerson/Blueprints/BP_ThirdPersonCharacter.BP_ThirdPersonCharacter_C|GetMaxHealth _playercharacter))
      (Default|HealPlayer _returnvalue_2 0.5)
      (Actor|DestroyActor))))

(event EventBeginPlay)

(event EventTick
  (params (DeltaSeconds :type Float%20%28single-precision%29)))

(fn ConstructionScript
  (bind _returnvalue (Rendering|Material|CreateDynamicMaterialInstance (Variables|Default|GetSphere) 0 "/Game/WorldObjects/M_DebugObjectColor.M_DebugObjectColor" "None" :!class /Script/Engine.PrimitiveComponent))
  (Rendering|Material|SetVectorParameterValue _returnvalue "Color" "(R=0.970578,G=1.000000,B=0.175239,A=1.000000)" :!class /Script/Engine.MaterialInstanceDynamic)
  (Rendering|Material|SetVectorParameterValue _returnvalue "EmissiveColor" "(R=1.000000,G=0.007234,B=0.000000,A=1.000000)" :!class /Script/Engine.MaterialInstanceDynamic)
  (Rendering|Material|SetScalarParameterValue _returnvalue "EmissiveMult" 2e+01 :!class /Script/Engine.MaterialInstanceDynamic))