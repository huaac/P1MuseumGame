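; BP_MeleeRobot is a flipbook-based melee robot enemy whose AI runs in a MeleeRobotAI state machine, created and started on BeginPlay.
; Pawn sensing sets the state machine's InCombat flag when it sees the player.
; Each tick it flips 180 degrees to face the player in combat, or its horizontal movement direction otherwise.
; A text render shows the flipbook's looping state, apparently for debugging.
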(event OnSeePawn(PawnSensing)
  (params (Pawn :type Pawn%20Object%20Reference))
  (if (== Pawn (Game|GetPlayerCharacter 0))
    (Variables|/Game/StateMachines/MeleeRobotAI.MeleeRobotAI_C|SetInCombat (Variables|Default|GetStateMachine) true)))

(event Custom|SetCharacterRotation
  (Rendering|Components|TextRender|SetText (Variables|Default|GetTextRender) (Utilities|Text|ToText(Boolean) (Class|PaperFlipbookComponent|IsLooping (Variables|Default|GetFlipbook))))
  (if (Variables|/Game/StateMachines/MeleeRobotAI.MeleeRobotAI_C|GetInCombat (Variables|Default|GetStateMachine))
    (if (>= (Math|Float|Absolute(Float) (.yaw (Math|Rotator|FindLookatRotation (Transformation|GetActorLocation) (Transformation|GetActorLocation (Game|GetPlayerCharacter 0))))) 9e+01)
      (Transformation|SetActorRotation "0.000000,180.000000,0.000000")
      (else
        (Transformation|SetActorRotation "0, 0, 0")))
    (else
      (Math|Float|CompareFloat (.x (Variables|/Script/Engine.MovementComponent|GetVelocity (Variables|Character|GetCharacterMovement))) 0.0
        (:>
          (Transformation|SetActorRotation (Math|Rotator|MakeRotator 0.0 0.0 0.0)))
        (:<
          (Transformation|SetActorRotation (Math|Rotator|MakeRotator 0.0 0.0 1.8e+02)))))))

(event EventBeginPlay
  (bind _returnvalue (Class|SMBlueprintUtils|CreateStateMachineInstance "/Game/StateMachines/MeleeRobotAI.MeleeRobotAI_C" self true))
  (bind _asmelee_robot_ai (Utilities|Casting|CastToMeleeRobotAI _returnvalue))
  (bind _output_get (Variables|Default|SetStateMachine _asmelee_robot_ai))
  (Class|SMInstance|Start _output_get))

(event Collision|EventActorBeginOverlap
  (params (OtherActor :type Actor%20Object%20Reference)))

(event EventTick
  (params (DeltaSeconds :type Float%20%28single-precision%29))
  (CallFunction|SetCharacterRotation))

(fn ConstructionScript)